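; Short-lived melee attack damage zone for the 2D platformer player, detecting hits through an overlap collision.
; On BeginPlay it caches the player character to read its current damage multiplier.
; When an overlapped actor carries the destroyable tag, it sends scaled damage through an interface message, spawns a hit effect and destroys itself.
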(event OnComponentBeginOverlap(Collision)
  (params (OverlappedComponent :type Primitive%20Component%20Object%20Reference) (OtherActor :type Actor%20Object%20Reference) (OtherComp :type Primitive%20Component%20Object%20Reference) (OtherBodyIndex :type Integer) (bFromSweep :type Boolean) (SweepResult :type Hit%20Result%20Structure%20%28by%20ref%29))
  ;[1 1 1] Spawn damage zone
  (if (Actor|ActorHasTag OtherActor (Variables|Default|GetDestroyableTag))
    ;;[0.1595 0.2271 1] Blueprint Interface Call
    (Class|InteractionHandler|ActorDamagedbyObject(Message) OtherActor (* (Variables|Default|GetDamage) (Variables|/Game/2DSideScrollerBP/Player_Character0.Player_Character0_C|GetCurrentDamageMultiplier (Variables|Default|GetPlayerReference))) "0, 0, 0")
    ;;[0.1595 0.2271 1] Spawn Hit FX
    (Effects|SpawnEmitteratLocation (Variables|Default|GetmeleeHitFX) (Transformation|GetWorldLocation (Variables|Default|GetCollision)))
    (Actor|DestroyActor)))

(event EventBeginPlay
  ;[1 1 1] Get player Reference
  (bind _asplayer_character_0 (Utilities|Casting|CastToPlayer_Character0 (Game|GetPlayerCharacter 0)))
  (Variables|Default|SetPlayerReference _asplayer_character_0))

(fn ConstructionScript)