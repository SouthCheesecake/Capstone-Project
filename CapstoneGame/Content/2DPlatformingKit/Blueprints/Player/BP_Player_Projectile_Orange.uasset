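; Orange player projectile Blueprint for the 2D platforming kit that deals damage on hit and then destroys itself.
; On collision it ignores the player and sends tagged destroyable actors an interface damage message scaled by the player's current damage multiplier, with a ranged hit effect.
; Any other hit spawns a generic impact effect and a half-scale ground impact sprite.
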(event OnComponentHit(Collision)
  (params (HitComponent :type Primitive%20Component%20Object%20Reference) (OtherActor :type Actor%20Object%20Reference) (OtherComp :type Primitive%20Component%20Object%20Reference) (NormalImpulse :type Vector :default "0, 0, 0") (Hit :type Hit%20Result%20Structure%20%28by%20ref%29))
  (bind _collision (Variables|Default|GetCollision))
  (bind _returnvalue (Transformation|GetWorldLocation _collision))
  ;[1 1 1] Player projectile hit
  ;;[0.1595 0.2271 1] Ignore the Player
  (if (not (== OtherActor (Game|GetPlayerCharacter 0)))
    (if (Actor|ActorHasTag OtherActor (Variables|Default|GetDestroyableTag))
      ;;[0.1595 0.2271 1] Blueprint Interface Call
      (Class|InteractionHandler|ActorDamagedbyObject(Message) OtherActor (* (Variables|Default|GetDamage) (Variables|/Game/2DSideScrollerBP/Player_Character0.Player_Character0_C|GetCurrentDamageMultiplier (Variables|Default|GetPlayerReference))) "0, 0, 0")
      ;;[0.1595 0.2271 1] Spawn Hit FX
      (Effects|SpawnEmitteratLocation (Variables|Default|GetrangedHitFX) (Transformation|GetWorldLocation (Variables|Default|GetCollision)))
      (Actor|DestroyActor)
      (else
        ;;[0.1595 0.2271 1] Spawn Ground Hit FX
        (Effects|SpawnEmitteratLocation (Variables|Default|GetgenericHitFX) _returnvalue)
        (Game|SpawnActorfromClass (Variables|Default|GetgroundImpactSprite) (Math|Transform|MakeTransform _returnvalue "0, 0, 0" "0.500000,0.500000,0.500000") "AdjustIfPossibleButDontSpawnIfColliding" 0 0)
        (Actor|DestroyActor)))))

(event EventBeginPlay
  ;[1 1 1] Get player Reference
  (bind _asplayer_character_0 (Utilities|Casting|CastToPlayer_Character0 (Game|GetPlayerCharacter 0)))
  (Variables|Default|SetPlayerReference _asplayer_character_0))

(fn ConstructionScript)